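; Cadeau2 is a gift actor that shakes, then turns into a random trap.
; On BeginPlay, a timeline's update adds X, Y and Z shake offsets to the Cube's current world location, with sweep.
; The same update chain runs into a one-second Delay, then spawns one of the first two TrapList classes at the Cube's transform and destroys the gift.
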(event EventBeginPlay
  (bind (_direction _shakex _shakey _shakez) (Timeline|Timeline_0 Play)
    (:Update
      (Transformation|SetWorldLocation (Variables|Default|GetCube) (+ (Transformation|GetWorldLocation (Variables|Default|GetCube)) (Math|Vector|MakeVector _shakex _shakey _shakez)) true false)
      (Utilities|FlowControl|Delay 1.0)
      (Game|SpawnActorfromClass (Utilities|Array|Get(acopy) (Variables|Default|GetTrapList) (Math|Random|RandomInteger 2)) (Transformation|GetWorldTransform (Variables|Default|GetCube)) "Undefined" 0 0)
      (Actor|DestroyActor))))

(event Collision|EventActorBeginOverlap
  (params (OtherActor :type Actor%20Object%20Reference)))

(event EventTick
  (params (DeltaSeconds :type Float%20%28single-precision%29)))

(fn ConstructionScript)