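; WaveSoundPlayer is a Blueprint that switches music between a between-wave theme and a wave theme.
; StartBetweenPhase plays the between-wave theme, which Tick replays whenever the audio stops during that phase.
; StartPhase stores the next wave sound and raises a flag, so Tick calls EndBetweenPhase to play it only after the current between-wave track finishes, avoiding a mid-track cut.
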(event Custom|StartBetweenPhase
  (bind _audio (Variables|Default|GetAudio))
  (Variables|Default|SetBetweenWave true)
  (Variables|Default|SetStartWave false)
  (Audio|Components|Audio|SetSound _audio (Variables|Default|GetSound_BetweenWave))
  (Audio|Components|Audio|Play _audio 0.0))

(event Custom|StartPhase
  (params (NewParam :type Sound%20Cue%20Object%20Reference))
  (Variables|Default|SetSoundWave NewParam)
  (Variables|Default|SetStartWave true))

(event Custom|EndBetweenPhase
  (bind _audio (Variables|Default|GetAudio))
  (Variables|Default|SetBetweenWave false)
  (Audio|Components|Audio|SetSound _audio (Variables|Default|GetSoundWave))
  (Audio|Components|Audio|Play _audio 0.0))

(event EventBeginPlay)

(event Collision|EventActorBeginOverlap
  (params (OtherActor :type Actor%20Object%20Reference)))

(event EventTick
  (params (DeltaSeconds :type Float%20%28single-precision%29))
  (if (Variables|Default|GetBetweenWave)
    (if (not (Audio|Components|Audio|IsPlaying (Variables|Default|GetAudio)))
      (if (Variables|Default|GetStartWave)
        ;[1 1 1] On joue le theme de la wave
        (CallFunction|EndBetweenPhase)
        (else
          ;[1 1 1] On joue le theme entre les wave en boucle
          (Audio|Components|Audio|Play (Variables|Default|GetAudio) 0.0))))))

(fn ConstructionScript)