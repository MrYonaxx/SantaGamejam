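; AI controller for enemies that starts the Enemy_BehaviorTree on BeginPlay and exposes helpers that write its TargetPosition and Target blackboard keys.
; SetPositions stores a list of waypoint actors and calls FindNextPosition, which writes the current actor's location to TargetPosition and advances the index.
; IsEndPosition reports true once the index is one past the list length, meaning FindNextPosition has run once after the last waypoint.
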(event EventBeginPlay
  (AI|RunBehaviorTree "/Game/Blueprints/Enemy/Enemy_BehaviorTree.Enemy_BehaviorTree"))

(event EventTick
  (params (DeltaSeconds :type Float%20%28single-precision%29)))

(fn ConstructionScript)

(fn SetPosition
  (params (Pos :type Vector))
  (AI|Components|Blackboard|SetValueasVector (AI|GetBlackboard 0) (Utilities|Name|MakeLiteralName "TargetPosition") Pos))

(fn SetTarget
  (params (TargetKdo :type Actor%20Object%20Reference))
  (AI|Components|Blackboard|SetValueasObject (AI|GetBlackboard 0) (Utilities|Name|MakeLiteralName "Target") TargetKdo))

(fn FindNextPosition
  (if (< (Variables|Default|GetIndexPosition) (Utilities|Array|Length (Variables|Default|GetListPosition)))
    (AI|Components|Blackboard|SetValueasVector (AI|GetBlackboard 0) (Utilities|Name|MakeLiteralName "TargetPosition") (Transformation|GetActorLocation (Utilities|Array|Get(acopy) (Variables|Default|GetListPosition) (Variables|Default|GetIndexPosition)))))
  (Math|Integer|IncrementInt (Variables|Default|GetIndexPosition)))

(fn IsEndPosition
  (return (== (Variables|Default|GetIndexPosition) (+ (Utilities|Array|Length (Variables|Default|GetListPosition)) 1))))

(fn SetPositions
  (params (NewParam :type Array%20of%20Actor%20Object%20References))
  (Variables|Default|SetListPosition NewParam)
  (CallFunction|FindNextPosition))