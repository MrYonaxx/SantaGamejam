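; Enemy character Blueprint that can be slowed or sped up, take damage, and attack a target by removing its gifts.
; It caches base walk speed on BeginPlay, and SetSpeed scales movement from that value.
; TakeDamage lowers Health, then fires the OnDeath dispatcher and destroys the actor at zero or below.
; SetAttack stores the target and flags attacking, while AttackTarget removes gifts by the Attack value and clears the flag.
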(event EventBeginPlay
  (Variables|Default|SetBaseSpeed (Variables|/Script/Engine.CharacterMovementComponent|GetMaxWalkSpeed (Variables|Character|GetCharacterMovement))))

(event Collision|EventActorBeginOverlap
  (params (OtherActor :type Actor%20Object%20Reference)))

(event EventTick
  (params (DeltaSeconds :type Float%20%28single-precision%29)))

(fn ConstructionScript)

(fn SetSpeed
  (params (SpeedMultiplier :type Float%20%28single-precision%29))
  (Variables|/Script/Engine.CharacterMovementComponent|SetMaxWalkSpeed (Variables|Character|GetCharacterMovement) (* (Variables|Default|GetBaseSpeed) SpeedMultiplier)))

(fn TakeDamage
  (params (Damage :type Integer))
  (bind _output_get (Variables|Default|SetHealth (- (Variables|Default|GetHealth) Damage)))
  (if (<= _output_get 0)
    (Default|CallOnDeathDispatcher)
    (Actor|DestroyActor)))

(fn SetAttack
  (params (AttackTarget :type Reserve%20Cadeau%20Object%20Reference))
  (Variables|Default|SetTarget AttackTarget)
  (Variables|Default|SetisAttacking true))

(fn AttackTarget
  (bind _target (Variables|Default|GetTarget))
  (Utilities|IsValid _target
    (:Is%20Valid
      (Default|RemoveGifts _target (Variables|Default|GetAttack))
      (Variables|Default|SetisAttacking false))))