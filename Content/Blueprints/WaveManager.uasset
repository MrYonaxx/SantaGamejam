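; WaveManager actor that runs successive enemy waves, switching music and showing a wave HUD.
; Each wave's DataTable rows time enemy spawns at random points in a box, giving AI controllers a target and random waypoint path.
; Death dispatchers feed a kill count; clearing a wave triggers brief slow motion, then the next wave after a delay or an empty win event.
; Between-wave music loops until spawning resumes, switching when the track ends.
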(event Custom|EnemyDeath
  ;[1 1 1] Enemy Death
  (Variables|Default|SetKillCount (+ (Variables|Default|GetKillCount) 1))
  (Development|PrintString "Enemy Dead")
  (if (not (Variables|Default|GetWaveInProgress))
    (if (== (Variables|Default|GetKillCount) (Variables|Default|GetMaxKillCount))
      (Development|PrintString "Next wave")
      (CallFunction|StartBetweenPhase)
      (Utilities|Time|SetGlobalTimeDilation 0.2)
      (Utilities|FlowControl|Delay 0.4)
      (Utilities|Time|SetGlobalTimeDilation 1.0)
      (if (== (Variables|Default|GetGlobalWaveIndex) (+ (Utilities|Array|Length (Variables|Default|GetGlobalWaveData)) -1))
        (CallFunction|EventWin)
        (else
          (Utilities|FlowControl|Delay (Variables|Default|GetTimeBetweenWave))
          (CallFunction|StartNewWave))))))

(event Custom|StartBetweenPhase
  (bind _audio (Variables|Default|GetAudio))
  ;[1 1 1] Sound
  (Variables|Default|SetBetweenWave true)
  (Audio|Components|Audio|SetSound _audio (Variables|Default|GetSoundBetweenWave))
  (Audio|Components|Audio|Play _audio 0.0))

(event Custom|EventStartWave
  (bind _hudwaveinstantiate (Variables|Default|GetHUDWaveInstantiate))
  (Widget|SetVisibility _hudwaveinstantiate "Visible")
  (bind _aswave_hud (Utilities|Casting|CastToWaveHUD _hudwaveinstantiate))
  (Default|DrawWave _aswave_hud (+ (Variables|Default|GetGlobalWaveIndex) 1))
  (Utilities|FlowControl|Delay 3.0)
  (Widget|SetVisibility _hudwaveinstantiate "Hidden"))

(event Custom|EventWin)

(event Custom|EndBetweenPhase
  (bind _audio (Variables|Default|GetAudio))
  ;[1 1 1] Sound
  (Variables|Default|SetBetweenWave false)
  (Audio|Components|Audio|SetSound _audio (.WaveBGM (Utilities|Struct|BreakGlobalWaveData (Utilities|Array|Get(acopy) (Variables|Default|GetGlobalWaveData) (Variables|Default|GetGlobalWaveIndex)))))
  (Audio|Components|Audio|Play _audio 0.0))

(event Custom|UpdateSound
  (params (DeltaSeconds :type Float%20%28single-precision%29))
  ;[1 1 1] Sound
  (if (Variables|Default|GetBetweenWave)
    (if (not (Audio|Components|Audio|IsPlaying (Variables|Default|GetAudio)))
      (if (Variables|Default|GetWaveInProgress)
        ;[1 1 1] On joue le theme de la wave
        (CallFunction|EndBetweenPhase)
        (else
          ;[1 1 1] On joue le theme entre les wave en boucle
          (Audio|Components|Audio|Play (Variables|Default|GetAudio) 0.0))))))

(event EventBeginPlay
  (CallFunction|StartBetweenPhase)
  (CallFunction|SelectWaveData)
  (bind _returnvalue (UserInterface|CreateWidget "/Game/Blueprints/UI/WaveHUD.WaveHUD_C" (Game|GetPlayerController 0)))
  (Variables|Default|SetHUDWaveInstantiate _returnvalue)
  (UserInterface|Viewport|AddtoViewport _returnvalue 0)
  (Utilities|FlowControl|Delay 3.0)
  (Widget|SetVisibility (Variables|Default|GetHUDWaveInstantiate) "Hidden"))

(event Collision|EventActorBeginOverlap
  (params (OtherActor :type Actor%20Object%20Reference)))

(event EventTick
  (params (DeltaSeconds :type Float%20%28single-precision%29))
  (bind _currentwavedata (Variables|Default|GetCurrentWaveData))
  (bind (_timespawn _enemytype _enemynumber) (Utilities|Struct|BreakWaveData _currentwavedata))
  (CallFunction|UpdateSound DeltaSeconds)
  (if (Variables|Default|GetWaveInProgress)
    (bind _output_get (Variables|Default|SetTImeWave (+ (Variables|Default|GetTImeWave) DeltaSeconds)))
    (if (>= _output_get _timespawn)
      (CallFunction|SpawnEnemy _enemytype _enemynumber)
      (Variables|Default|SetWaveIndex (+ (Variables|Default|GetWaveIndex) 1))
      (CallFunction|SelectWaveData))))

(fn ConstructionScript)

(fn SpawnEnemy
  (params (EnemyID :type Integer) (EnemyNumber :type Integer))
  (bind _boxspawn (Variables|Default|GetBoxSpawn))
  (bind _destination (Variables|Default|GetDestination))
  (for _index (range 1 EnemyNumber)
    (bind _returnvalue (Game|SpawnActorfromClass (Utilities|Array|Get(acopy) (Variables|Default|GetEnemyDatabase) EnemyID) (Math|Conversions|ToTransform(Vector) (Math|Random|RandomPointinBoundingBox (Transformation|GetWorldLocation _boxspawn) (Components|Box|GetScaledBoxExtent _boxspawn))) "AdjustIfPossibleButAlwaysSpawn" 0 0))
    (EventDispatchers|BindEventtoOnDeathDispatcher _returnvalue (EventDispatchers|CreateEvent :!event Custom|EnemyDeath))
    (bind _asenemy_aicontroller (Utilities|Casting|CastToEnemy_AIController (AI|GetAIController _returnvalue)))
    (Default|SetTarget _asenemy_aicontroller _destination)
    (Default|SetPositions _asenemy_aicontroller (Variables|/Game/Blueprints/WavePath.WavePath_C|GetWaypoints (Utilities|Array|Get(acopy) (Variables|Default|GetWavePaths) (Math|Random|RandomIntegerinRange 0 (- (Utilities|Array|Length (Variables|Default|GetWavePaths)) 1)))) _destination)
    (Variables|Default|SetMaxKillCount (+ (Variables|Default|GetMaxKillCount) 1))))

(fn SelectWaveData
  (bind _outrownames (DataTable|GetDataTableRowNames (.GlobalWaveData (Utilities|Struct|BreakGlobalWaveData (Utilities|Array|Get(acopy) (Variables|Default|GetGlobalWaveData) (Variables|Default|GetGlobalWaveIndex))))))
  (for (_array_element _array_index) _outrownames
    (if (== _array_index (Variables|Default|GetWaveIndex))
      (bind _returnvalue (Utilities|GetDataTableRow (.GlobalWaveData (Utilities|Struct|BreakGlobalWaveData (Utilities|Array|Get(acopy) (Variables|Default|GetGlobalWaveData) (Variables|Default|GetGlobalWaveIndex)))) _array_element)
        (:then
          (Variables|Default|SetCurrentWaveData _returnvalue)
          (Variables|Default|SetWaveInProgress true)
          (return)))))
  (Development|PrintString "EndWave")
  (Variables|Default|SetWaveInProgress false))

(fn StartNewWave
  (Variables|Default|SetTImeWave 0.0)
  (Variables|Default|SetWaveIndex 0)
  (Variables|Default|SetKillCount 0)
  (Variables|Default|SetMaxKillCount 0)
  (Variables|Default|SetGlobalWaveIndex (+ (Variables|Default|GetGlobalWaveIndex) 1))
  (CallFunction|SelectWaveData)
  (CallFunction|EventStartWave))