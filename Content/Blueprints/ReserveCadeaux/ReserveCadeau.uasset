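; Gift reserve actor that serves as the life pool: running out of gifts means defeat.
; On BeginPlay it fills the count, adds the ammo and health bar widgets, and scatters gift actors with random materials inside its box.
; RemoveGifts lowers the count, destroys only the last listed gift per call, then checks for defeat, which pauses the game and shows the defeat screen.
; Overlap events flag whether the first-person character is inside the zone.
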(event Custom|SpawnLifePoints
  (bind _box (Variables|Default|GetBox))
  ;[1 1 1] SpawnGiftLifePoints
  (for _index (range 1 (Variables|Default|GetMaxCadeaux))
    (Variables|Default|SetRdmMaterial (Math|Random|RandomInteger 3))
    (bind _returnvalue (Game|SpawnActorfromClass (Variables|Default|GetGiftList) (Math|Conversions|ToTransform(Vector) (Math|Random|RandomPointinBoundingBox (Transformation|GetWorldLocation _box) (Components|Box|GetScaledBoxExtent _box))) "AlwaysSpawn" 0 0))
    (Utilities|Array|AddUnique (Variables|Default|GetInstantiateGiftList) _returnvalue)
    (bind _asgift_life_points (Utilities|Casting|CastToGiftLifePoints _returnvalue))
    (Rendering|Material|SetMaterial (Variables|/Game/Blueprints/ReserveCadeaux/GiftLifePoints.GiftLifePoints_C|GetCube _asgift_life_points) 0 (Utilities|Array|Get(acopy) (Variables|Default|GetGiftMaterialList) (Variables|Default|GetRdmMaterial)))))

(event EventBeginPlay
  (Utilities|FlowControl|Sequence
    (:then_0
      (Variables|Default|SetCurrentCadeaux (Variables|Default|GetMaxCadeaux)))
    (:then_1
      (bind _returnvalue (UserInterface|CreateWidget "/Game/Blueprints/ZoneAmmo/UIAmmo.UIAmmo_C"))
      (UserInterface|Viewport|AddtoViewport _returnvalue 0))
    (:then_2
      (bind _returnvalue_2 (UserInterface|CreateWidget "/Game/Blueprints/UI/HealthBar.HealthBar_C"))
      (UserInterface|Viewport|AddtoViewport _returnvalue_2 0))
    (:then_3
      (CallFunction|SpawnLifePoints))))

(event Collision|EventActorBeginOverlap
  (params (OtherActor :type Actor%20Object%20Reference))
  (bind _asfirst_person_character (Utilities|Casting|CastToFirstPersonCharacter OtherActor))
  (Variables|/Game/FirstPersonBP/Blueprints/FirstPersonCharacter.FirstPersonCharacter_C|SetisInReserveCadeauZone _asfirst_person_character true)
  (Variables|Default|SetplayerInZone true))

(event EventTick
  (params (DeltaSeconds :type Float%20%28single-precision%29)))

(event Collision|EventActorEndOverlap
  (params (OtherActor :type Actor%20Object%20Reference))
  (bind _asfirst_person_character (Utilities|Casting|CastToFirstPersonCharacter OtherActor))
  (Variables|/Game/FirstPersonBP/Blueprints/FirstPersonCharacter.FirstPersonCharacter_C|SetisInReserveCadeauZone _asfirst_person_character false)
  (Variables|Default|SetplayerInZone false))

(fn ConstructionScript)

(fn RemoveGifts
  (params (numberOfGifts :type Integer))
  (bind _instantiategiftlist (Variables|Default|GetInstantiateGiftList))
  (bind _returnvalue (Utilities|Array|Length _instantiategiftlist))
  (bind _returnvalue_2 (- _returnvalue 1))
  (Variables|Default|SetCurrentCadeaux (- (Variables|Default|GetCurrentCadeaux) numberOfGifts))
  (Actor|DestroyActor (Utilities|Array|Get(acopy) _instantiategiftlist _returnvalue_2))
  (Utilities|Array|RemoveIndex _instantiategiftlist _returnvalue_2)
  (CallFunction|DefeatChecker))

(fn SpawnGiftLifePoint)

(fn DefeatChecker
  (bind _returnvalue (Game|GetPlayerController 0))
  (if (<= (Variables|Default|GetCurrentCadeaux) 0)
    (Game|SetGamePaused true)
    (Viewport|RemoveAllWidgets)
    (Variables|/Script/Engine.PlayerController|SetbShowMouseCursor _returnvalue true)
    (bind _returnvalue_2 (UserInterface|CreateWidget "/Game/Blueprints/FinishScreens/DefeatScreen.DefeatScreen_C" _returnvalue))
    (Input|SetInputModeUIOnly _returnvalue _returnvalue_2 "DoNotLock")
    (UserInterface|Viewport|AddtoViewport _returnvalue_2 0)))